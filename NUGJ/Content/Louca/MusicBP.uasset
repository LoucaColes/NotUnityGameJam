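; MusicBP is an actor that plays the Pegboard Nerds Heartbit music cue and bends its pitch to match a Spline's frequency.
; BeginPlay sets the pitch to normal and starts playback.
; Each Tick converts the Spline's Frequency to a pitch, with 50 mapping to normal pitch, and updates the cue's pitch multiplier only when that value changes.
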(event `self.ReceiveBeginPlay`
  (bind _pegboard_nerds___heartbit_cue (`self.Pegboard_Nerds_-_Heartbit_Cue`))
  ;[1 1 1] Set pitch to 1 and play music
  (bind _output_get (set `self.pitch` 1.0))
  (`AudioComponent.SetPitchMultiplier` _pegboard_nerds___heartbit_cue _output_get)
  (`AudioComponent.Play` _pegboard_nerds___heartbit_cue 0.0))

(event `self.ReceiveTick`
  (params (DeltaSeconds :type "Float (single-precision)"))
  (bind _returnvalue (* 2 (/ (`/Game/Louca/SplineBP.Frequency` (`self.Spline`)) 100.0)))
  (if (!= (`self.pitch`) _returnvalue)
    ;[1 1 1] If there was update the pitch multiplier
    (bind _output_get (set `self.pitch` _returnvalue))
    (`AudioComponent.SetPitchMultiplier` (`self.Pegboard_Nerds_-_Heartbit_Cue`) _output_get)))

(fn `UserConstructionScript`)