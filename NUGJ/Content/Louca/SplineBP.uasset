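; SplineBP is an actor that draws an endlessly extending, scrolling spline strip from spline mesh components.
; Tick moves the spline and meshes along negative X, and every half second appends a point, trims the oldest beyond Limit, and rebuilds all meshes.
; New point height is Amplitude times the sine of frame delta times Frequency, not elapsed time.
; Each tick also creates dynamic material instances to apply two lerp parameters; destroyed meshes are never cleared from the array.
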(event `self.ReceiveBeginPlay`
  (set `self.Made` false)
  (set `self.NewVar_3` 0)
  (set `self.timer` 0.0)
  (`self.CreateSpline`))

(event `self.ReceiveTick`
  (params (DeltaSeconds :type "Float (single-precision)"))
  (`self.ChangeMatColour` (`self.TestLerpOne`) (`self.TestLerpTwo`))
  (`self.MoveSpline` DeltaSeconds)
  (set `self.timer` (+ DeltaSeconds (`self.timer`)))
  (if (>= (`self.timer`) 0.5)
    (set `self.timer` 0.0)
    (bind _output_get (set `self.NewVar_3` (+ (`self.NewVar_3`) 1)))
    (`SplineComponent.AddPoint` (`self.Spline`) (make `SplinePoint` (`KismetMathLibrary.Conv_IntToDouble` _output_get) (`KismetMathLibrary.MakeVector` (`KismetMathLibrary.Conv_IntToDouble` (+ 100 (* _output_get (`KismetMathLibrary.FTrunc` (`self.Frequency`))))) 0.0 (* (`KismetMathLibrary.Sin` (* DeltaSeconds (`self.Frequency`))) (`self.Amplitude`))) (50.0 0.0 50.0) (50.0 0.0 50.0) (struct) (1.0 1.0 1.0)) true)
    (`self.RemovePoint`)
    (`self.DeleteSpline`)
    (`self.CreateSpline`)))

(fn `ChangeMatColour`
  (params (LerpOne :type "Float (double-precision)") (LerpTwo :type "Float (double-precision)"))
  (locals (SplineMeshComp :type "SplineMeshComponent Object Reference") (TLerpOne :type "Float (double-precision)") (TLerpTwo :type "Float (double-precision)"))
  (bind _output_get (set `local.TLerpOne` LerpOne))
  (set `self.TestLerpOne` _output_get)
  (bind _output_get_2 (set `local.TLerpTwo` LerpTwo))
  (set `self.TestLerpTwo` _output_get_2)
  (for _array_element (`self.smcs`)
    (bind _output_get_3 (set `local.SplineMeshComp` _array_element))
    (if (`KismetSystemLibrary.IsValid` _output_get_3)
      (bind _returnvalue (`PrimitiveComponent.CreateDynamicMaterialInstance` (`local.SplineMeshComp`) 0 "/Game/Louca/SplineMat.SplineMat"))
      (`MaterialInstanceDynamic.SetScalarParameterValue` _returnvalue "LerpOne" (`local.TLerpOne`))
      (`MaterialInstanceDynamic.SetScalarParameterValue` _returnvalue "LerpTwo" (`local.TLerpTwo`))))
  (return))

(fn `CreateMeshComp`
  (params (StartPos :type "Vector Structure") (StartTan :type "Vector Structure") (EndPos :type "Vector Structure") (EndTan :type "Vector Structure"))
  (bind _returnvalue (`AddComponent|NODE_AddSplineMeshComponent-5` :`RelativeTransform` (`SceneComponent.GetRelativeTransform` (`self.Spline`))))
  (`self.ChangeMatColour` (`self.TestLerpOne`) (`self.TestLerpTwo`))
  (`KismetArrayLibrary.Array_Add` (`self.smcs`) _returnvalue)
  (`SceneComponent.K2_AttachToComponent` _returnvalue (`self.DefaultSceneRoot`) "None" "KeepRelative" "KeepRelative" "KeepRelative" true)
  (`SplineMeshComponent.SetStartAndEnd` _returnvalue StartPos StartTan EndPos EndTan true)
  (return))

(fn `CreateSpline`
  (bind _spline (`self.Spline`))
  (for _index (range (`self.NewVar_0`) (+ (- (`SplineComponent.GetNumberOfSplinePoints` (`self.Spline`)) 2) 1))
    (bind (_location _tangent) (`SplineComponent.GetLocationAndTangentAtSplinePoint` _spline _index "Local"))
    (bind (_location_2 _tangent_2) (`SplineComponent.GetLocationAndTangentAtSplinePoint` _spline (+ _index 1) "Local"))
    (`self.CreateMeshComp` _location _tangent _location_2 _tangent_2)))

(fn `DeleteSpline`
  (for _array_element (`self.smcs`)
    (if (`KismetSystemLibrary.IsValid` _array_element)
      (`ActorComponent.K2_DestroyComponent` _array_element)))
  (return))

(fn `MoveSpline`
  (params (DeltaTime :type "Float (double-precision)"))
  (locals (DeltaX :type "Float (double-precision)" :default 0.0))
  (bind _output_get (set `local.DeltaX` (* DeltaTime (* (`self.MoveSpeed`) -1.0))))
  (`SceneComponent.K2_AddRelativeLocation` (`self.Spline`) (`KismetMathLibrary.MakeVector` _output_get) false false)
  (for _array_element (`self.smcs`)
    (if (`KismetSystemLibrary.IsValid` _array_element)
      (`SceneComponent.K2_AddRelativeLocation` _array_element (`KismetMathLibrary.MakeVector` (`local.DeltaX`)) false false)))
  (return))

(fn `RemovePoint`
  (if (> (`SplineComponent.GetNumberOfSplinePoints` (`self.Spline`)) (`self.Limit`))
    (`SplineComponent.RemoveSplinePoint` (`self.Spline`) 0 true)
    (return)))

(fn `UserConstructionScript`
  (locals (NewLocalVar_0 :type Integer :default 0)))