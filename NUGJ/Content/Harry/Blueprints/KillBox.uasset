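; KillBox is an actor that acts as a fall-death zone beneath the player, following them horizontally at a set height.
; On BeginPlay it attaches to the first player controller's pawn.
; Each Tick it teleports its root to that pawn's X and Y, with Z held at DeathHeight.
; When a Player overlaps its Box, it calls TakeDamage on that Player with a fixed, presumably lethal, amount.
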(event `self.ReceiveBeginPlay`
  (`self.K2_AttachToActor` (`Controller.K2_GetPawn` (`GameplayStatics.GetPlayerController` 0)) "None" "KeepRelative" "KeepRelative" "KeepRelative"))

(event `self.Box.OnComponentBeginOverlap`
  (params (OverlappedComponent :type "PrimitiveComponent Object Reference") (OtherActor :type "Actor Object Reference") (OtherComp :type "PrimitiveComponent Object Reference") (OtherBodyIndex :type Integer) (bFromSweep :type Boolean) (SweepResult :type "HitResult Structure (by ref)"))
  (bind _asplayer (cast `/Game/Harry/Blueprints/Player` OtherActor))
  (`/Game/Harry/Blueprints/Player.TakeDamage` _asplayer 100.0))

(event `self.ReceiveTick`
  (params (DeltaSeconds :type "Float (single-precision)"))
  (bind _returnvalue (`Controller.K2_GetPawn` (`GameplayStatics.GetPlayerController` 0)))
  (if (`KismetSystemLibrary.IsValid` _returnvalue)
    (`SceneComponent.K2_SetWorldLocation` (`self.DefaultSceneRoot`) (`KismetMathLibrary.MakeVector` (.x (`self.K2_GetActorLocation` _returnvalue)) (.y (`self.K2_GetActorLocation` _returnvalue)) (`self.DeathHeight`)) false true)))

(fn `UserConstructionScript`)