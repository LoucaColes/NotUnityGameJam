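; HeartRunner is a Blueprint that spawns a row of Collectable actors when play begins.
; BeginPlay loops to place nine collectables evenly along the world X axis at a fixed height, giving each random Positive, Negative and Player values.
; AddCollectable spawns each actor at its position and passes those three values to the Collectable's SetSectionsSizes.
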(event `self.ReceiveBeginPlay`
  (for _index (range -4 5)
    (`self.AddCollectable` (`KismetMathLibrary.MakeVector` (* _index 100.0) 0.0 100.0) (`KismetMathLibrary.RandomFloatInRange` 0.0 10.0) (`KismetMathLibrary.RandomFloatInRange` 0.0 10.0) (`KismetMathLibrary.RandomFloatInRange` 0.0 10.0))))

(fn `AddCollectable`
  (params (Position :type "Vector Structure") (Positive :type "Float (double-precision)") (Negative :type "Float (double-precision)") (Player :type "Float (double-precision)"))
  (bind _returnvalue (`|SpawnActorFromClass` "/Game/Harry/Blueprints/Collectable.Collectable_C" (`KismetMathLibrary.Conv_VectorToTransform` Position) "Undefined" "OverrideRootScale" null null))
  (bind _ascollectable (cast `/Game/Harry/Blueprints/Collectable` _returnvalue))
  (`/Game/Harry/Blueprints/Collectable.SetSectionsSizes` _ascollectable Positive Negative Player))

(fn `UserConstructionScript`)