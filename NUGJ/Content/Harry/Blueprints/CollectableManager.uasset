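; CollectableManager spawns Collectable actors at the end of a referenced Spline as that end point changes.
; On Tick, a countdown gates a position check that negates the last point's X, then adds the spline actor's location and a spawn offset.
; If that position differs from the previous spawn, AddCollectable spawns a Collectable with random Positive, Negative and Player section sizes, passes it the Spline, and the timer resets.
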(event `self.ReceiveTick`
  (params (DeltaSeconds :type "Float (single-precision)"))
  (bind _lastpos (`/Game/Louca/SplineBP.GetLastPos` (`self.Spline`)))
  (bind _output_get (set `self.TimeRemaining` (- (`self.TimeRemaining`) DeltaSeconds)))
  (if (<= _output_get 0.0)
    (bind _returnvalue (+ (+ (`KismetMathLibrary.MakeVector` (* -1 (.x _lastpos)) (.y _lastpos) (.z _lastpos)) (`self.K2_GetActorLocation` (`self.Spline`))) (`self.SpawnOffset`)))
    (if (!= _returnvalue (`self.LastPosition`))
      (bind _output_get_2 (set `self.LastPosition` _returnvalue))
      (`self.AddCollectable` _output_get_2 (`KismetMathLibrary.RandomFloatInRange` 0.0 10.0) (`KismetMathLibrary.RandomFloatInRange` 0.0 10.0) (`KismetMathLibrary.RandomFloatInRange` 0.0 10.0))
      (set `self.TimeRemaining` (`self.SpawnWait`)))))

(fn `AddCollectable`
  (params (Position :type "Vector Structure") (Positive :type "Float (double-precision)") (Negative :type "Float (double-precision)") (Player :type "Float (double-precision)"))
  (bind _returnvalue (`|SpawnActorFromClass` "/Game/Harry/Blueprints/Collectable.Collectable_C" (`KismetMathLibrary.Conv_VectorToTransform` Position) "Undefined" "OverrideRootScale" null null))
  (`/Game/Harry/Blueprints/Collectable.SetSectionsSizes` _returnvalue Positive Negative Player)
  (`/Game/Harry/Blueprints/Collectable.SetSplineRef` _returnvalue (`self.Spline`)))

(fn `UserConstructionScript`)